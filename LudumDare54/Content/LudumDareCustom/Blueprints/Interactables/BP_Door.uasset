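; BP_Door is an interactable hinged door that alternately opens and closes each time InteractEvent fires.
; On opening, a dot product of the interactor's capsule forward vector and the door's Arrow picks the swing direction, so it follows the way the interactor faces.
; The DoorOpen timeline scales a quarter-turn yaw on the door mesh, and a FlipFlop plays or reverses it.
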(event EventBeginPlay)

(event Collision|EventActorBeginOverlap
  (params (OtherActor :type Actor%20Object%20Reference)))

(event EventTick
  (params (DeltaSeconds :type Float%20%28single-precision%29))
  (|CallParentFunction DeltaSeconds) ; This node is disabled and will not be called.\nDrag off pins to build functionality.
)

(event EventInteractEvent
  (params (Interactor :type Character%20Object%20Reference))
  (Utilities|FlowControl|FlipFlop
    (:A
      (Variables|Default|SetOpenDirection (>= (Math|Vector|DotProduct (Math|Vector|GetForwardVector (Variables|/Script/Engine.Character|GetCapsuleComponent Interactor)) (Math|Vector|GetForwardVector (Variables|Default|GetArrow))) 0.0))
      (bind _scale (Timeline|DoorOpen Play)
        (:Update
          (Transformation|SetRelativeRotation (Variables|Default|GetStaticMesh) (Math|Rotator|MakeRotator 0.0 0.0 (* _scale (Math|Float|SelectFloat 9e+01 -9e+01 (Variables|Default|GetOpenDirection)))) false false))))
    (:B
      (Timeline|DoorOpen Reverse))))

(fn ConstructionScript
  (|CallParentFunction))